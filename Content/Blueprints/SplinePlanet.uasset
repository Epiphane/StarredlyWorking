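; SplinePlanet is a planet actor that can be placed along its PathPreview path for a given time.
; SetTime composes the transform stored at BeginPlay with the path's local-space transform at that time and applies it without sweep or teleport.
; Each tick, it copies the SimulatePhysics setting from OrbitPlayerControllerBP to its static mesh, while that controller is valid.
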(event EventBeginPlay
  (|CallParentFunction)
  (Variables|Default|SetInitial%20Transform (Transformation|GetActorTransform))
  (bind _asorbit_player_controller_bp (Utilities|Casting|CastToOrbitPlayerControllerBP (Game|GetPlayerController 0)))
  (bind _output_get (Variables|Default|SetPlayer%20Controller _asorbit_player_controller_bp))
  (Physics|SetSimulatePhysics (Variables|Default|GetStaticMesh) (Variables|/Game/Blueprints/GameMode/OrbitPlayerControllerBP.OrbitPlayerControllerBP_C|GetSimulatePhysics _output_get)))

(event EventTick
  (params (DeltaSeconds :type Float%20%28single-precision%29))
  (bind _player_controller (Variables|Default|GetPlayer%20Controller)
    (:then
      (Physics|SetSimulatePhysics (Variables|Default|GetStaticMesh) (Variables|/Game/Blueprints/GameMode/OrbitPlayerControllerBP.OrbitPlayerControllerBP_C|GetSimulatePhysics _player_controller)))
    (:else)))

(event EventSetTime
  (params (CurrentTime :type Float%20%28single-precision%29))
  (Transformation|SetActorTransform (Math|Transform|ComposeTransforms (Variables|Default|GetInitial%20Transform) (Spline|GetTransformatTime (Variables|Default|GetPathPreview) CurrentTime "Local" false false))))

(fn ConstructionScript
  (|CallParentFunction))