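; Enemy shooter that rides on a co-located pullable simulated body and fires bullet bursts at the player spaceship.
; Its mesh is offset by angle and radius, and while physics simulates it follows that owner each tick.
; A range and line-of-sight check feeds a lock timer that fills or decays.
; Once locked, it fires until empty, using the same timer for fire rate, then reloads and must lock again.
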(event EventBeginPlay
  (bind _self self)
  (|CallParentFunction)
  (Utilities|FlowControl|Sequence
    (:then_0
      ;[1 1 1] Sets closest orbiting Sim Body as owner
      (bind _outactors (Actor|GetAllActorsOfClass "/Game/Blueprints/SpaceObjects/BP_SimulatedBody.BP_SimulatedBody_C"))
      (for _array_element _outactors
        (if (!= _array_element _self)
          (if (and (Utilities|Operators|EqualEqual (Transformation|GetActorLocation _self) (Transformation|GetActorLocation _array_element) 1.0) (Variables|/Script/StarredlyWorking.GravityMovementComponent|GetbCanBePulled (Variables|/Game/Blueprints/SpaceObjects/BP_SimulatedBody.BP_SimulatedBody_C|GetGravityMovement _array_element)))
            (Actor|SetOwner _array_element)))))
    (:then_1
      (bind _outactors_2 (Actor|GetAllActorsOfClass "/Game/Blueprints/PlayerObjects/BP_ControlledBody.BP_ControlledBody_C"))
      (Variables|Default|SetAll%20Controlled%20Bodies%20Ref _outactors_2)
      (bind _outactors_3 (Actor|GetAllActorsOfClass "/Game/Blueprints/SpaceObjects/BP_FixedBody.BP_FixedBody_C"))
      (Variables|Default|SetAll%20Fixed%20Bodies%20Ref _outactors_3))
    (:then_2
      (Variables|Default|SetCurrent%20Rounds (Variables|Default|GetRound%20Capacity)))))

(event EventTick
  (params (DeltaSeconds :type Float%20%28single-precision%29))
  (if (Physics|IsSimulatingPhysics (Variables|Default|GetStaticMesh) "None")
    (Transformation|SetActorLocation (Transformation|GetActorLocation (Components|GetOwner)) false false)
    (bind (_is_targeting _spaceship) (CallFunction|GetLOStoTarget))
    (CallFunction|UpdateLockProgress _is_targeting DeltaSeconds)
    (CallFunction|FiringSequence _spaceship)))

(fn ConstructionScript
  (bind _radius (Variables|Default|GetRadius))
  (bind _angle (Variables|Default|GetAngle))
  (|CallParentFunction)
  (Transformation|SetRelativeTransform (Variables|Default|GetEnemyMesh) (Math|Transform|MakeTransform (Math|Vector|MakeVector (* (Math|Trig|Cos(Degrees) _angle) _radius) (* (Math|Trig|Sin(Degrees) _angle) _radius) 0.0) "-90.000000,0.000000,0.000000" "1.000000,1.000000,1.000000") false false))

(fn GetLOStoTarget
  (bind _enemymesh (Variables|Default|GetEnemyMesh))
  (bind _all_controlled_bodies_ref (Variables|Default|GetAll%20Controlled%20Bodies%20Ref))
  (bind _returnvalue (Transformation|GetWorldLocation _enemymesh))
  (bind _outactors (Actor|GetAllActorsOfClass "/Game/Blueprints/PlayerObjects/BP_Spaceship.BP_Spaceship_C"))
  (for _array_element _outactors
    (if (not (Variables|/Script/Engine.Actor|GetbHidden _array_element))
      (bind _returnvalue_2 (Collision|LineTraceByChannel _returnvalue (Transformation|GetActorLocation _array_element) "TraceTypeQuery1" false _all_controlled_bodies_ref "None"))
      (if (and (<= (Math|Vector|Distance(Vector) _returnvalue (Transformation|GetActorLocation _array_element)) (Variables|Default|GetRange)) (== _returnvalue_2 false))
        ;[1 0 0] Fix this messy shit...
        (Collision|LineTraceByChannel _returnvalue (Transformation|GetActorLocation _array_element) "TraceTypeQuery1" false _all_controlled_bodies_ref "ForOneFrame")
        (return true _array_element)
        (else
          (return false _array_element))))))

(fn UpdateLockProgress
  (params (Is%20Targeting :type Boolean) (Delta%20Seconds :type Float%20%28double-precision%29))
  ;[1 1 1] Keep incrementing time when in firing sequence
  (if (or Is%20Targeting (Variables|Default|GetIs%20Firing))
    (Variables|Default|SetCurrent%20Seconds (+ (Variables|Default|GetCurrent%20Seconds) Delta%20Seconds))
    ;[1 1 1] Begin firing sequence once locked
    (if (>= (Variables|Default|GetCurrent%20Seconds) (Variables|Default|GetSeconds%20to%20Target%20Lock))
      (Variables|Default|SetIs%20Firing true))
    (else
      (Variables|Default|SetCurrent%20Seconds (Math|Float|Max(Float) (- (Variables|Default|GetCurrent%20Seconds) Delta%20Seconds) 0.0))
      ;[1 1 1] Reload if t=0
      (if (<= (Variables|Default|GetCurrent%20Seconds) 0.0)
        (Variables|Default|SetCurrent%20Rounds (Variables|Default|GetRound%20Capacity))))))

(fn FiringSequence
  (params (Spaceship :type Actor%20Object%20Reference))
  ;[1 1 1] Stop firing if no ammo
  (if (<= (Variables|Default|GetCurrent%20Rounds) 0)
    (Variables|Default|SetCurrent%20Seconds 0.0)
    (Variables|Default|SetCurrent%20Rounds (Variables|Default|GetRound%20Capacity))
    (Variables|Default|SetIs%20Firing false)
    (else
      ;[1 1 1] Keep firing (at RPS rate) once started
      (if (and (Variables|Default|GetIs%20Firing) (>= (Variables|Default|GetCurrent%20Seconds) (Variables|Default|GetSeconds%20to%20Target%20Lock)))
        (Game|SpawnActorfromClass "/Game/Blueprints/SpaceObjects/BP_EnemyBullet.BP_EnemyBullet_C" (Math|Transform|MakeTransform (Transformation|GetWorldLocation (Variables|Default|GetEnemyMesh)) "0, 0, 0" "1.000000,1.000000,1.000000") "Undefined" "MultiplyWithRoot" self Spaceship (Variables|Default|GetBullet%20Velocity) (Variables|Default|GetBullet%20Spread%20%28Deg%29) (Variables|Default|GetAll%20Fixed%20Bodies%20Ref) 0)
        ;[1 1 1] Subtract RPS "cooldown" and decrement rounds
        (Variables|Default|SetCurrent%20Seconds (- (Variables|Default|GetCurrent%20Seconds) (Math|Float|SafeDivide 1.0 (Variables|Default|GetRounds%20per%20Second))))
        (Variables|Default|SetCurrent%20Rounds (- (Variables|Default|GetCurrent%20Rounds) 1))))))

(fn OnReset
  (params (Is%20Full%20Reset :type Boolean))
  (Variables|Default|SetCurrent%20Rounds (Variables|Default|GetRound%20Capacity))
  (Variables|Default|SetCurrent%20Seconds 0.0))