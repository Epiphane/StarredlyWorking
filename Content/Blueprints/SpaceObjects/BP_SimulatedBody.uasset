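; Simulated space body in an orbit game that starts with initial linear and angular velocity and can jump to any cached simulation time.
; SetTime reads SimulationCache to place the actor, then overwrites velocities on its physics-simulating meshes.
; It spawns configured attached bodies, passing angle and mesh radius, on BeginPlay and on full resets from the orbit player controller.
; GetInstantVelocity exposes current body velocity and initial spin.
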(event EventBeginPlay
  (Utilities|FlowControl|Sequence
    (:then_0
      ;[1 1 1] Initial physics state
      (Physics|AddImpulse (Variables|Default|GetStaticMesh) (Variables|Default|GetInitial%20Velocity) "None" true)
      (Class|PrimitiveComponent|SetAllPhysicsAngularVelocityinDegrees (Variables|Default|GetStaticMesh) (Variables|Default|GetInitial%20Angular%20Velocity) false))
    (:then_1
      ;[1 1 1] Assign custom launch behavior
      (bind _asbp_orbit_player_controller (Utilities|Casting|CastToBP_OrbitPlayerController (Game|GetPlayerController 0)))
      (bind _output_get (Variables|Default|SetPlayer%20Controller _asbp_orbit_player_controller))
      (EventDispatchers|BindEventtoOnLaunch _output_get (EventDispatchers|CreateEvent :!event OnLaunch))
      (EventDispatchers|BindEventtoOnReset _output_get (EventDispatchers|CreateEvent :!event OnReset))
      (CallFunction|SpawnAttachedBodies))))

(event EventSetTime
  (params (CurrentTime :type Float%20%28single-precision%29))
  (CallFunction|SetTimeInternal CurrentTime))

(fn ConstructionScript)

(fn SpawnAttachedBodies
  (for _array_element (Variables|Default|GetAttached%20Bodies)
    (Game|SpawnActorfromClass (.attachment _array_element) (Math|Transform|MakeTransform (Transformation|GetActorLocation) "-90.000000,0.000000,0.000000" "1.000000,1.000000,1.000000") "Undefined" "MultiplyWithRoot" self (.initialangledegrees _array_element) (* (.sphereradius (StaticMesh|GetBounds (Variables|/Script/Engine.StaticMeshComponent|GetStaticMesh (Variables|Default|GetStaticMesh)))) (Math|Vector|GetMaxElement (Transformation|GetActorScale3D))) 0)))

(fn GetInstantVelocity
  (return (Variables|Default|GetInitial%20Angular%20Velocity) (Variables|Default|GetCurrent%20Velocity)))

(fn SetTimeInternal
  (params (Time :type Float%20%28double-precision%29))
  (bind _simulationcache (Variables|Default|GetSimulationCache))
  (bind _outstate (Class|SimulationCacheComponent|GetStateatTime _simulationcache Time))
  (Utilities|FlowControl|Sequence
    (:then_0
      (Variables|Default|SetCurrent%20Velocity (.velocity _outstate))
      (Transformation|SetActorLocationAndRotation (.position _outstate) (Class|KismetMathLibrary|QuatRotator (.rotation _outstate))))
    (:then_1
      (for _array_element (Actor|GetComponentsByClass "/Script/Engine.StaticMeshComponent")
        (if (Physics|IsSimulatingPhysics _array_element "None")
          (Class|PrimitiveComponent|SetAllPhysicsLinearVelocity _array_element "0, 0, 0" false)
          (Physics|AddImpulse _array_element (.velocity _outstate) "None" true)
          (Class|PrimitiveComponent|SetPhysicsAngularVelocityinDegrees _array_element (.angularvelocity _outstate) false "None"))))))

(fn OnLaunch)

(fn OnReset
  (params (Is%20Full%20Reset :type Boolean))
  (if Is%20Full%20Reset
    (CallFunction|SpawnAttachedBodies)))