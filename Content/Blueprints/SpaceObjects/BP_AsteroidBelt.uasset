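; Asteroid belt actor that scatters static mesh asteroids around its origin in a flat, procedurally generated field.
; The construction script loops over the asteroid count, adding one static mesh component per pass.
; X and Y come from cosine and sine of random angles times random radii within the belt's range, with random per-axis scale.
; All random values draw from the Seed stream, and BeginPlay only calls the parent.
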(event EventBeginPlay
  (|CallParentFunction))

(event Collision|EventActorBeginOverlap
  (params (OtherActor :type Actor%20Object%20Reference)))

(event EventTick
  (params (DeltaSeconds :type Float%20%28single-precision%29)))

(fn ConstructionScript
  (bind _seed (Variables|Default|GetSeed))
  (bind _min_scale (Variables|Default|GetMin%20Scale))
  (bind _scale_range (Variables|Default|GetScale%20Range))
  (bind _min_radius (Variables|Default|GetMin%20Radius))
  (bind _radius_range (Variables|Default|GetRadius%20Range))
  (bind _returnvalue (Math|Random|RandomFloatinRangefromStream _seed 0.0 3.6e+02))
  (bind _returnvalue_2 (+ _min_radius _radius_range))
  (bind _returnvalue_3 (+ _min_scale _scale_range))
  (bind _returnvalue_4 (Math|Random|RandomFloatinRangefromStream _seed _min_scale _returnvalue_3))
  (bind _returnvalue_5 (Math|Random|RandomFloatinRangefromStream _seed _min_radius _returnvalue_2))
  (|CallParentFunction)
  (for _index (range 0 (Variables|Default|GetNumber%20of%20Asteroids))
    (AddComponent|AddStaticMeshComponent false (Math|Transform|MakeTransform (Math|Vector|MakeVector (* (Math|Trig|Cos(Degrees) _returnvalue) _returnvalue_5) (* (Math|Trig|Sin(Degrees) _returnvalue) _returnvalue_5) 0.0) "0, 0, 0" (Math|Vector|MakeVector _returnvalue_4 _returnvalue_4 _returnvalue_4)))))