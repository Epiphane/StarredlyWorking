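; Enemy bullet that launches at a target with a lead angle and hides itself and any spaceship it overlaps.
; On BeginPlay it solves an intercept yaw from relative velocity using the law of sines, adds random spread, then applies an impulse including the grand-owner's velocity.
; It finds the closest fixed body, but the aim calculation ignores that gravity source.
; The player controller's OnReset event destroys the bullet.
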(event EventBeginPlay
  (Utilities|FlowControl|Sequence
    (:then_0
      (bind _asbp_orbit_player_controller (Utilities|Casting|CastToBP_OrbitPlayerController (Game|GetPlayerController 0)))
      (EventDispatchers|BindEventtoOnReset _asbp_orbit_player_controller (EventDispatchers|CreateEvent :!event OnReset)))
    (:then_1
      (bind _fixed_body (CallFunction|FindClosestFixedBody)))
    (:then_2
      (bind _firing_vector (CallFunction|CalculateFiringAngle _fixed_body))
      (Physics|AddImpulse (Variables|Default|GetStaticMesh) (+ (* _firing_vector (Variables|Default|GetVelocity)) (Transformation|GetVelocity (Components|GetOwner (Components|GetOwner)))) "None" true)
      (Transformation|SetActorRotation (Math|Rotator|MakeRotator 0.0 -9e+01 (.yaw (Math|Rotator|FindLookatRotation (Transformation|GetActorLocation self) (Transformation|GetActorLocation (Variables|Default|GetTarget)))))))))

(event EventTick
  (params (DeltaSeconds :type Float%20%28single-precision%29))
  (for _array_element (Collision|GetOverlappingActors (Variables|Default|GetBox) "/Game/Blueprints/PlayerObjects/BP_Spaceship.BP_Spaceship_C" :!class /Script/Engine.PrimitiveComponent)
    (Utilities|IsValid _array_element
      (:Is%20Valid
        (Rendering|SetActorHiddenInGame _array_element true)
        (Rendering|SetActorHiddenInGame true)))))

(fn ConstructionScript)

(fn OnReset
  (params (Is%20Full%20Reset :type Boolean))
  (Actor|DestroyActor))

(fn CalculateFiringAngle
  (params (Gravity%20Source :type Actor%20Object%20Reference))
  (bind _returnvalue (Transformation|GetActorLocation))
  (bind _returnvalue_2 (Components|GetOwner))
  (bind _target (Variables|Default|GetTarget))
  (bind _spread__deg_ (Variables|Default|GetSpread%20%28Deg%29))
  (bind _returnvalue_3 (Transformation|GetVelocity _target))
  (bind _returnvalue_4 (Transformation|GetActorLocation _target))
  (bind _returnvalue_5 (Components|GetOwner _returnvalue_2))
  (bind _returnvalue_6 (Transformation|GetVelocity _returnvalue_5))
  (bind _returnvalue_7 (- _returnvalue_4 _returnvalue))
  (bind _returnvalue_8 (Class|KismetMathLibrary|VectorHeadingAngle _returnvalue_7))
  (bind _returnvalue_9 (* _returnvalue_6 -1.0))
  (bind _returnvalue_10 (Math|Trig|RadiansToDegrees _returnvalue_8))
  (bind _returnvalue_11 (+ _returnvalue_9 _returnvalue_3))
  (bind _returnvalue_12 (Class|KismetMathLibrary|VectorHeadingAngle _returnvalue_11))
  (bind _returnvalue_13 (>= _returnvalue_10 0.0))
  (bind _returnvalue_14 (Math|Trig|RadiansToDegrees _returnvalue_12))
  (return (Class|KismetMathLibrary|CreateVectorfromYawPitch (+ (Math|Random|RandomFloatinRange (* _spread__deg_ -1.0) _spread__deg_) (+ (* (Class|KismetMathLibrary|DegAsin (/ (Math|Vector|VectorLength _returnvalue_11) (/ (Variables|Default|GetVelocity) (Math|Trig|Sin(Degrees) (Math|Float|Absolute(Float) (- 1.8e+02 (Math|Float|Absolute(Float) (- _returnvalue_14 _returnvalue_10)))))))) (* (Math|Float|SelectFloat -1.0 1.0 (Math|Float|InRange(Float) _returnvalue_14 (- _returnvalue_10 (Math|Float|SelectFloat 1.8e+02 0.0 _returnvalue_13)) (+ _returnvalue_10 (Math|Float|SelectFloat 0.0 1.8e+02 _returnvalue_13)))) (Math|Float|SelectFloat 1.0 -1.0 _returnvalue_13))) _returnvalue_10)) 0.0 1.0)))

(fn FindClosestFixedBody
  (for _array_element (Variables|Default|GetAll%20Fixed%20Bodies%20Ref)
    (if (< (Transformation|GetDistanceTo _array_element) (LocalVariables|GetLeast%20Distance))
      (LocalVariables|SetLeast%20Distance (Transformation|GetDistanceTo _array_element))
      (LocalVariables|SetClosest%20Body _array_element)))
  (return (LocalVariables|GetClosest%20Body)))