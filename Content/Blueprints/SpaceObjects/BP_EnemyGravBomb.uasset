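; Enemy gravity bomb projectile that spawns a BP_GravityWell with DetonationMass when its timer runs out, then destroys itself.
; On BeginPlay it computes a lead angle from Target and firing ship (owner's owner) velocities, adds random spread and launches by impulse.
; The same trigonometric intercept sets the detonation time, ignoring gravity: the closest fixed body is passed in but unused.
; The player controller's reset event also destroys it.
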(event EventBeginPlay
  (Utilities|FlowControl|Sequence
    (:then_0
      (bind _asbp_orbit_player_controller (Utilities|Casting|CastToBP_OrbitPlayerController (Game|GetPlayerController 0)))
      (EventDispatchers|BindEventtoOnReset _asbp_orbit_player_controller (EventDispatchers|CreateEvent :!event OnReset)))
    (:then_1
      (bind _fixed_body (CallFunction|FindClosestFixedBody)))
    (:then_2
      (bind _firing_vector (CallFunction|CalculateDetonationLocation _fixed_body))
      (Physics|AddImpulse (Variables|Default|GetStaticMesh) (+ (* _firing_vector (Variables|Default|GetVelocity)) (Transformation|GetVelocity (Components|GetOwner (Components|GetOwner)))) "None" true)
      (Transformation|SetActorRotation (Math|Rotator|MakeRotator 0.0 -9e+01 (.yaw (Math|Rotator|FindLookatRotation (Transformation|GetActorLocation self) (Transformation|GetActorLocation (Variables|Default|GetTarget)))))))))

(event EventTick
  (params (DeltaSeconds :type Float%20%28single-precision%29))
  (bind _output_get (Variables|Default|SetTime%20to%20Detonate (Math|Float|Max(Float) (- (Variables|Default|GetTime%20to%20Detonate) DeltaSeconds) 0.0)))
  (if (<= _output_get 0.0)
    (Game|SpawnActorfromClass "/Game/Blueprints/SpaceObjects/BP_GravityWell.BP_GravityWell_C" (Math|Transform|MakeTransform (Transformation|GetActorLocation) "0, 0, 0" "1.000000,1.000000,1.000000") "Undefined" "MultiplyWithRoot" 0 (Variables|Default|GetDetonation%20Mass) 0)
    (Actor|DestroyActor)))

(fn ConstructionScript)

(fn OnReset
  (params (Is%20Full%20Reset :type Boolean))
  (Actor|DestroyActor))

(fn CalculateDetonationLocation
  (params (Gravity%20Source :type Actor%20Object%20Reference))
  (bind _returnvalue (Transformation|GetActorLocation))
  (bind _returnvalue_2 (Components|GetOwner))
  (bind _target (Variables|Default|GetTarget))
  (bind _spread__deg_ (Variables|Default|GetSpread%20%28Deg%29))
  (bind _velocity (Variables|Default|GetVelocity))
  (bind _returnvalue_3 (Transformation|GetVelocity _target))
  (bind _returnvalue_4 (Transformation|GetActorLocation _target))
  (bind _returnvalue_5 (Components|GetOwner _returnvalue_2))
  (bind _returnvalue_6 (Transformation|GetVelocity _returnvalue_5))
  (bind _returnvalue_7 (- _returnvalue_4 _returnvalue))
  (bind _returnvalue_8 (Class|KismetMathLibrary|VectorHeadingAngle _returnvalue_7))
  (bind _returnvalue_9 (* _returnvalue_6 -1.0))
  (bind _returnvalue_10 (Math|Trig|RadiansToDegrees _returnvalue_8))
  (bind _returnvalue_11 (+ _returnvalue_9 _returnvalue_3))
  (bind _returnvalue_12 (Class|KismetMathLibrary|VectorHeadingAngle _returnvalue_11))
  (bind _returnvalue_13 (Math|Vector|VectorLength _returnvalue_11))
  (bind _returnvalue_14 (>= _returnvalue_10 0.0))
  (bind _returnvalue_15 (Math|Trig|RadiansToDegrees _returnvalue_12))
  (bind _returnvalue_16 (- _returnvalue_15 _returnvalue_10))
  (bind _returnvalue_17 (Math|Float|Absolute(Float) _returnvalue_16))
  (bind _returnvalue_18 (- 1.8e+02 _returnvalue_17))
  (bind _returnvalue_19 (Math|Float|Absolute(Float) _returnvalue_18))
  (bind _returnvalue_20 (Math|Trig|Sin(Degrees) _returnvalue_19))
  (bind _returnvalue_21 (/ _velocity _returnvalue_20))
  (bind _returnvalue_22 (/ _returnvalue_13 _returnvalue_21))
  (bind _returnvalue_23 (Class|KismetMathLibrary|DegAsin _returnvalue_22))
  (Variables|Default|SetTime%20to%20Detonate (/ (Math|Vector|VectorLength _returnvalue_7) (* (Math|Trig|Sin(Degrees) (+ _returnvalue_19 _returnvalue_23)) _returnvalue_21)))
  (return (Class|KismetMathLibrary|CreateVectorfromYawPitch (+ (Math|Random|RandomFloatinRange (* _spread__deg_ -1.0) _spread__deg_) (+ (* _returnvalue_23 (* (Math|Float|SelectFloat -1.0 1.0 (Math|Float|InRange(Float) _returnvalue_15 (- _returnvalue_10 (Math|Float|SelectFloat 1.8e+02 0.0 _returnvalue_14)) (+ _returnvalue_10 (Math|Float|SelectFloat 0.0 1.8e+02 _returnvalue_14)))) (Math|Float|SelectFloat 1.0 -1.0 _returnvalue_14))) _returnvalue_10)) 0.0 1.0)))

(fn FindClosestFixedBody
  (for _array_element (Variables|Default|GetAll%20Fixed%20Bodies%20Ref)
    (if (< (Transformation|GetDistanceTo _array_element) (LocalVariables|GetLeast%20Distance))
      (LocalVariables|SetLeast%20Distance (Transformation|GetDistanceTo _array_element))
      (LocalVariables|SetClosest%20Body _array_element)))
  (return (LocalVariables|GetClosest%20Body)))