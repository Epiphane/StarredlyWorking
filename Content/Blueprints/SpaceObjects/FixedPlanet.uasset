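; FixedPlanet is a space-object actor that records its motion history and can be moved to a chosen moment in it.
; Tick uses a Delay to sample location and velocity into arrays at tenth-second intervals until a simulated-time cap.
; Once enough time is recorded, SetTime teleports the planet to the indexed position.
; If GravityMovement allows pulling, it also applies the stored velocity as a mass-independent impulse to the static mesh.
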(event EventTick
  (params (DeltaSeconds :type Float%20%28single-precision%29))
  (bind _returnvalue (Transformation|GetVelocity))
  (if (< (Variables|Default|GetSimulatedTime) 61.0)
    (Utilities|FlowControl|Delay 0.1)
    (Variables|Default|SetSimulatedTime (+ (Variables|Default|GetSimulatedTime) 0.1))
    (Utilities|Array|Add (Variables|Default|GetArrayPositions) (Transformation|GetActorLocation))
    (Utilities|Array|Add (Variables|Default|GetArrayVelocities) _returnvalue)
    (Development|PrintString (Utilities|String|ToString(Vector) _returnvalue))))

(event Collision|EventActorBeginOverlap
  (params (OtherActor :type Actor%20Object%20Reference)))

(event EventSetTime
  (params (CurrentTime :type Float%20%28single-precision%29))
  (bind _returnvalue (* CurrentTime 1e+01))
  (bind _arrayvelocities (Variables|Default|GetArrayVelocities))
  (bind _returnvalue_2 (Math|Float|Round _returnvalue))
  (bind _output (Utilities|Array|Get(acopy) _arrayvelocities _returnvalue_2))
  (if (not (< (Variables|Default|GetSimulatedTime) 21.0))
    (Utilities|FlowControl|Sequence
      (:then_0
        (Transformation|SetActorLocation (Utilities|Array|Get(acopy) (Variables|Default|GetArrayPositions) _returnvalue_2) false false)
        (goto _label Open))
      (:then_1
        (if (Variables|/Script/StarredlyWorking.GravityMovementComponent|GetbCanBePulled (Variables|Default|GetGravityMovement))
          (Utilities|FlowControl|Gate true :!label _label
            (:Exit
              (Physics|AddImpulse (Actor|GetComponentbyClass "/Script/Engine.StaticMeshComponent") _output "None" true)
              (Development|PrintString (Utilities|String|ToString(Vector) _output)))))))))

(fn ConstructionScript
  (|CallParentFunction))