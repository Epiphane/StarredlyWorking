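; Enemy seeker turret that rides on a pullable simulated body and fires one homing-style missile at the player spaceship per reset.
; It adopts the co-located body as owner at BeginPlay and follows it while simulating physics, with its mesh offset by Angle and Radius.
; Range and line-of-sight checks, ignoring controlled bodies, build or decay a lock timer.
; A reticle on the ship shrinks until lock spawns BP_EnemyMissile.
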(event EventBeginPlay
  (bind _self self)
  (|CallParentFunction)
  (Utilities|FlowControl|Sequence
    (:then_0
      ;[1 1 1] Sets closest orbiting Sim Body as owner
      (bind _outactors (Actor|GetAllActorsOfClass "/Game/Blueprints/SpaceObjects/BP_SimulatedBody.BP_SimulatedBody_C"))
      (for _array_element _outactors
        (if (!= _array_element _self)
          (if (and (Utilities|Operators|EqualEqual (Transformation|GetActorLocation _self) (Transformation|GetActorLocation _array_element) 1.0) (Variables|/Script/StarredlyWorking.GravityMovementComponent|GetbCanBePulled (Variables|/Game/Blueprints/SpaceObjects/BP_SimulatedBody.BP_SimulatedBody_C|GetGravityMovement _array_element)))
            (Actor|SetOwner _array_element)))))
    (:then_1
      (bind _outactors_2 (Actor|GetAllActorsOfClass "/Game/Blueprints/PlayerObjects/BP_ControlledBody.BP_ControlledBody_C"))
      (Variables|Default|SetAll%20Controlled%20Bodies%20Ref _outactors_2))))

(event EventTick
  (params (DeltaSeconds :type Float%20%28single-precision%29))
  (bind _seconds_to_target_lock (Variables|Default|GetSeconds%20to%20Target%20Lock))
  (bind _current_seconds (Variables|Default|GetCurrent%20Seconds))
  (bind _returnvalue (- _seconds_to_target_lock _current_seconds))
  (if (Physics|IsSimulatingPhysics (Variables|Default|GetStaticMesh) "None")
    (Transformation|SetActorLocation (Transformation|GetActorLocation (Components|GetOwner)) false false)
    (if (Variables|Default|GetIs%20Loaded)
      (bind (_is_targeting _spaceship) (CallFunction|GetLOStoTarget))
      (CallFunction|UpdateLockProgress _is_targeting _spaceship DeltaSeconds)
      (Transformation|SetWorldScale3D (Variables|Default|GetReticleMesh) (Math|Vector|MakeVector _returnvalue _returnvalue _returnvalue))
      (else
        (Rendering|SetVisibility (Variables|Default|GetReticleMesh) false false)))))

(fn ConstructionScript
  (bind _radius (Variables|Default|GetRadius))
  (bind _angle (Variables|Default|GetAngle))
  (|CallParentFunction)
  (Transformation|SetRelativeTransform (Variables|Default|GetEnemyMesh) (Math|Transform|MakeTransform (Math|Vector|MakeVector (* (Math|Trig|Cos(Degrees) _angle) _radius) (* (Math|Trig|Sin(Degrees) _angle) _radius) 0.0) "-90.000000,0.000000,0.000000" "1.000000,1.000000,1.000000") false false))

(fn GetLOStoTarget
  (bind _enemymesh (Variables|Default|GetEnemyMesh))
  (bind _returnvalue (Transformation|GetWorldLocation _enemymesh))
  (bind _outactors (Actor|GetAllActorsOfClass "/Game/Blueprints/PlayerObjects/BP_Spaceship.BP_Spaceship_C"))
  (for _array_element _outactors
    (if (not (Variables|/Script/Engine.Actor|GetbHidden _array_element))
      (Transformation|SetWorldLocation (Variables|Default|GetReticleMesh) (Transformation|GetActorLocation _array_element) false false)
      (bind _returnvalue_2 (Collision|LineTraceByChannel _returnvalue (Transformation|GetActorLocation _array_element) "TraceTypeQuery1" false (Variables|Default|GetAll%20Controlled%20Bodies%20Ref) "None"))
      (if (and (<= (Math|Vector|Distance(Vector) _returnvalue (Transformation|GetActorLocation _array_element)) (Variables|Default|GetRange)) (== _returnvalue_2 false))
        (return true _array_element)
        (else
          (return false _array_element))))))

(fn UpdateLockProgress
  (params (Is%20Targeting :type Boolean) (Spaceship :type Actor%20Object%20Reference) (Delta%20Seconds :type Float%20%28double-precision%29))
  (if Is%20Targeting
    (Variables|Default|SetCurrent%20Seconds (+ (Variables|Default|GetCurrent%20Seconds) Delta%20Seconds))
    (Rendering|SetVisibility (Variables|Default|GetReticleMesh) true false)
    (if (>= (Variables|Default|GetCurrent%20Seconds) (Variables|Default|GetSeconds%20to%20Target%20Lock))
      (Variables|Default|SetIs%20Loaded false)
      (Variables|Default|SetCurrent%20Seconds 0.0)
      (Game|SpawnActorfromClass "/Game/Blueprints/SpaceObjects/BP_EnemyMissile.BP_EnemyMissile_C" (Math|Transform|MakeTransform (Transformation|GetWorldLocation (Variables|Default|GetEnemyMesh)) "0, 0, 0" "1.000000,1.000000,1.000000") "Undefined" "MultiplyWithRoot" self Spaceship (Variables|Default|GetMissile%20Acceleration) (Variables|Default|GetMissile%20Flight%20Time) 0))
    (else
      (Variables|Default|SetCurrent%20Seconds (Math|Float|Max(Float) (- (Variables|Default|GetCurrent%20Seconds) Delta%20Seconds) 0.0))
      (if (<= (Variables|Default|GetCurrent%20Seconds) 0.0)
        (Rendering|SetVisibility (Variables|Default|GetReticleMesh) false false)))))

(fn OnReset
  (params (Is%20Full%20Reset :type Boolean))
  (Variables|Default|SetIs%20Loaded true)
  (Variables|Default|SetCurrent%20Seconds 0.0))