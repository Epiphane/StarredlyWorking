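; Player-launched spaceship for an orbit game, with an adjustable launch angle that wraps within a full circle.
; On BeginPlay it increases its ControllerDist and binds to the OrbitPlayerControllerBP's OnLaunch dispatcher.
; On launch it clears its owner, enables physics on its mesh and applies a mass-independent impulse along the angle in the XY plane, scaled by LaunchSpeed.
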(event Custom|Modify%20Launch%20Angle
  (params (Change :type Float%20%28double-precision%29))
  (CallFunction|SetAngle (Class|KismetMathLibrary|FWrap (+ (* Change 2.0) (Variables|Default|GetAngle)) 0.0 3.6e+02)))

(event EventBeginPlay
  (Variables|Default|SetControllerDist (+ (Variables|Default|GetControllerDist) 65.0))
  ;[1 1 1] Listen for Launch
  (bind _asorbit_player_controller_bp (Utilities|Casting|CastToOrbitPlayerControllerBP (Game|GetPlayerController 0)))
  (EventDispatchers|BindEventtoOnLaunch _asorbit_player_controller_bp (EventDispatchers|CreateEvent :!event OnLaunch)))

(fn ConstructionScript
  (|CallParentFunction))

(fn OnLaunch
  (bind _staticmesh (Variables|Default|GetStaticMesh))
  (bind _angle (Variables|Default|GetAngle))
  (Actor|SetOwner 0)
  (Physics|SetSimulatePhysics _staticmesh true)
  (Physics|AddImpulse _staticmesh (* (Math|Vector|MakeVector (Math|Trig|Cos(Degrees) _angle) (Math|Trig|Sin(Degrees) _angle) 0.0) (Variables|Default|GetLaunchSpeed)) "None" true))