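; BP_ControlledBody is a player-object actor that sits at a launch angle around its owner and listens to the orbit player controller.
; On BeginPlay and restore it binds to BP_OrbitPlayerController's launch and reset events, and on remove it unbinds them.
; SetLaunchAngle uses sine and cosine to position it on an XY circle around the owner, rotated to match the angle.
; Its OnLaunch and OnReset functions are empty.
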(event EventBeginPlay
  (Class|GravityActor|OnRestore))

(event EventOnRemove
  (bind _asbp_orbit_player_controller (Utilities|Casting|CastToBP_OrbitPlayerController (Game|GetPlayerController 0)))
  (EventDispatchers|UnbindEventfromOnLaunch _asbp_orbit_player_controller (EventDispatchers|CreateEvent :!event OnLaunch))
  (EventDispatchers|UnbindEventfromOnReset _asbp_orbit_player_controller (EventDispatchers|CreateEvent :!event OnReset)))

(event EventOnRestore
  (bind _asbp_orbit_player_controller (Utilities|Casting|CastToBP_OrbitPlayerController (Game|GetPlayerController 0)))
  (EventDispatchers|BindEventtoOnLaunch _asbp_orbit_player_controller (EventDispatchers|CreateEvent :!event OnLaunch))
  (EventDispatchers|BindEventtoOnReset _asbp_orbit_player_controller (EventDispatchers|CreateEvent :!event OnReset)))

(fn ConstructionScript)

(fn SetLaunchAngle
  (params (New%20Angle :type Float%20%28double-precision%29))
  (bind _controllerdist (Variables|Default|GetControllerDist))
  (bind _returnvalue (+ _controllerdist 65.0))
  (bind _output_get (Variables|Default|SetAngle New%20Angle))
  (Transformation|SetActorLocationAndRotation (+ (Transformation|GetActorLocation (Components|GetOwner)) (Math|Vector|MakeVector (* (Math|Trig|Cos(Degrees) _output_get) _returnvalue) (* _returnvalue (Math|Trig|Sin(Degrees) _output_get)) 0.0)) (Math|Rotator|MakeRotator 0.0 2.7e+02 _output_get)))

(fn OnLaunch)

(fn OnReset
  (params (Is%20Full%20Reset :type Boolean)))