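; BP_RCSComponent is an actor component that gives its owner fuel-limited reaction control thrusters for rotating and pushing it.
; Input burns fuel per frame, applying angular impulse about the owner's forward axis and linear impulse along its up vector, both scaled by fuel burned and thrust.
; It shows a fuel widget in a HUD slot and refills on the orbit controller's launch event; its reset handler's logic is disconnected.
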(event Custom|Set%20RCS%20Input
  (params (Yaw%20Input :type Float%20%28double-precision%29) (Thrust%20Input :type Float%20%28double-precision%29))
  (if (> (Variables|Default|GetFuel%20Level) 0.0)
    (CallFunction|FireRCS Yaw%20Input Thrust%20Input)))

(event EventOnRestore
  (CallFunction|SetHUDSlot "NewEnumerator3" (Variables|Default|GetFuel%20Level%20UI)))

(event EventOnRemove
  (CallFunction|RemovefromHUD "NewEnumerator3" (Variables|Default|GetFuel%20Level%20UI)))

(event EventBeginPlay
  (bind _asbp_orbit_player_controller (Utilities|Casting|CastToBP_OrbitPlayerController (Game|GetPlayerController 0)))
  (bind _returnvalue (UserInterface|CreateWidget "/Game/Widgets/HUD/WBP_RCSFuelLevel.WBP_RCSFuelLevel_C" _asbp_orbit_player_controller _asbp_orbit_player_controller self))
  (bind _output_get (Variables|Default|SetFuel%20Level%20UI _returnvalue))
  (CallFunction|SetHUDSlot "NewEnumerator3" _output_get)
  (EventDispatchers|BindEventtoOnReset _asbp_orbit_player_controller (EventDispatchers|CreateEvent :!event OnReset))
  (EventDispatchers|BindEventtoOnLaunch _asbp_orbit_player_controller (EventDispatchers|CreateEvent :!event OnLaunch)))

(fn OnReset
  (params (Is%20Full%20Reset :type Boolean)))

(fn OnLaunch
  (Variables|Default|SetFuel%20Level (Variables|Default|GetInitial%20Fuel%20Level)))

(fn FireRCS
  (params (Rotation :type Float%20%28double-precision%29) (Thrust :type Float%20%28double-precision%29))
  (bind _returnvalue (Components|GetOwner))
  (bind _returnvalue_2 (Actor|GetComponentbyClass _returnvalue "/Script/Engine.PrimitiveComponent"))
  (bind _returnvalue_3 (Transformation|GetActorRotation _returnvalue))
  ;[1 1 1] Reduce Fuel Level
  (LocalVariables|SetReal%20Amount (- (Variables|Default|GetFuel%20Level) (Math|Float|Max(Float) (- (Variables|Default|GetFuel%20Level) (* (Variables|Default|GetFuel%20Burn%20Rate) (Utilities|Time|GetWorldDeltaSeconds))) 0.0)))
  (Variables|Default|SetFuel%20Level (Math|Float|Max(Float) (- (Variables|Default|GetFuel%20Level) (* (Variables|Default|GetFuel%20Burn%20Rate) (Utilities|Time|GetWorldDeltaSeconds))) 0.0))
  ;[1 1 1] Get vector from actor and apply torque
  (Class|PrimitiveComponent|AddAngularImpulseinDegrees _returnvalue_2 (* (Math|Vector|GetForwardVector _returnvalue_3) (LocalVariables|GetReal%20Amount) (Variables|Default|GetThrust) (* Rotation -1.0)) "None" false)
  (if (> Thrust 0.0)
    (Physics|AddImpulse _returnvalue_2 (* (Math|Vector|GetUpVector _returnvalue_3) (LocalVariables|GetReal%20Amount) (/ (Variables|Default|GetThrust) 1e+02)) "None" false)))