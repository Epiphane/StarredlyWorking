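; Player spaceship that sits on a planet at an adjustable launch angle, then becomes a physics-driven craft on launch.
; BeginPlay spawns a RocketBooster at every mesh socket.
; Before launch, Tick re-applies the angle to track the planet and angle input moves it; afterwards, the same input drives RCS rotation.
; On launch it enables physics and inherits the owning SimulatedBody's velocity, spin and tangential surface speed.
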(event Custom|Modify%20Angle
  (params (Sign :type Float%20%28double-precision%29) (Triggered%20Seconds :type Float%20%28double-precision%29))
  (if (not (Variables|Default|GetbHidden))
    (if (Physics|IsSimulatingPhysics (Variables|Default|GetStaticMesh) "None")
      (Default|RCSRotation (Variables|Default|GetRCSComponent) Sign)
      (else
        (CallFunction|SetLaunchAngle (Class|KismetMathLibrary|FWrap (+ (* (* Sign Triggered%20Seconds) 2.0) (Variables|Default|GetAngle)) 0.0 3.6e+02))))))

(event EventBeginPlay
  (|CallParentFunction)
  (CallFunction|SetLaunchAngle (Variables|Default|GetAngle))
  (for _array_element (Transformation|GetAllSocketNames (Variables|Default|GetStaticMesh))
    (bind _returnvalue (Game|SpawnActorfromClass "/Game/Blueprints/PlayerObjects/RocketBooster.RocketBooster_C" (Math|Transform|MakeTransform "0, 0, 0" "0, 0, 0" "1.000000,1.000000,1.000000") "Undefined" "MultiplyWithRoot" 0 0.0 0.0 0))
    (Transformation|AttachActorToActor _returnvalue self _array_element "SnapToTarget" "SnapToTarget" "KeepWorld" true)))

(event EventTick
  (params (DeltaSeconds :type Float%20%28single-precision%29))
  ;[1 1 1] Constantly updates position to attached planet pre-launch
  (if (not (Physics|IsSimulatingPhysics (Variables|Default|GetStaticMesh) "None"))
    (CallFunction|SetLaunchAngle (Variables|Default|GetAngle))))

(fn ConstructionScript
  (|CallParentFunction))

(fn OnLaunch
  (bind _angle (Variables|Default|GetAngle))
  (bind _staticmesh (Variables|Default|GetStaticMesh))
  (|CallParentFunction)
  (Physics|SetSimulatePhysics _staticmesh true)
  (bind _assimulated_body (Utilities|Casting|CastToSimulatedBody (Components|GetOwner))
    (:then
      (bind (_surface_angular_velocity _body_velocity) (Default|GetInstantVelocity _assimulated_body)))
    (:CastFailed
      _))
  (Class|PrimitiveComponent|AddTorqueinDegrees _staticmesh _surface_angular_velocity "None" true)
  (Physics|AddImpulse _staticmesh (+ _body_velocity (* (Math|Vector|MakeVector (* (Math|Trig|Sin(Degrees) _angle) -1.0) (Math|Trig|Cos(Degrees) _angle) 0.0) (* (/ (/ (.Z (Math|Vector|BreakVector _surface_angular_velocity)) 1e+02) 3.6e+02) (Math|Float|MultiplybyPi (* (Variables|Default|GetControllerDist) 2.0))))) "None" true))