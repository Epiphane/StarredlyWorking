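; TEST_ShipCamera is a test camera actor that trails its owner and pairs a scene capture with an on-screen ship indicator widget.
; BeginPlay creates a render target for the capture and passes it to a TEST_ShipIndicator.
; Tick interpolates toward the owner and updates the indicator's direction from the view center; its visibility check yields HitTestInvisible either way.
; Actor and widget are removed once the owner is invalid.
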(event EventBeginPlay
  (bind _scenecapturecomponent2d (Variables|Default|GetSceneCaptureComponent2D))
  (bind _texturetarget (Variables|/Script/Engine.SceneCaptureComponent2D|GetTextureTarget _scenecapturecomponent2d))
  (Variables|Default|SetTarget (Components|GetOwner))
  (Rendering|CreateAndAssignRenderTarget _texturetarget 512 512 "RTF_RGBA16f"
    (:Out
      (bind _returnvalue (UserInterface|CreateWidget "/Game/Widgets/HUD/TEST_ShipIndicator.TEST_ShipIndicator_C" (Game|GetPlayerController 0) _texturetarget))
      (bind _output_get (Variables|Default|SetIndicator _returnvalue))
      (Widget|SetVisibility _output_get "Collapsed")
      (UserInterface|Viewport|AddtoViewport _output_get 0)
      (Default|SetDirectiontoTarget _output_get (- (Transformation|GetActorLocation) (.Center (CallFunction|GetPlayerViewBounds)))))))

(event EventTick
  (params (DeltaSeconds :type Float%20%28single-precision%29))
  (bind _indicator (Variables|Default|GetIndicator))
  (bind _target (Variables|Default|GetTarget)
    (:then
      (Transformation|SetActorLocation (Math|Interpolation|VInterpTo (Transformation|GetActorLocation) (Transformation|GetActorLocation _target) DeltaSeconds 0.0) false false)
      (Widget|SetVisibility _indicator (select (or (CallFunction|IsPointinViewport (Transformation|GetActorLocation _target)) (Variables|/Script/Engine.Actor|GetbHidden _target)) "HitTestInvisible" "HitTestInvisible"))
      (Default|SetDirectiontoTarget _indicator (- (Transformation|GetActorLocation) (.Center (CallFunction|GetPlayerViewBounds)))))
    (:else
      (Widget|RemovefromParent (Variables|Default|GetIndicator))
      (Actor|DestroyActor))))

(fn ConstructionScript)