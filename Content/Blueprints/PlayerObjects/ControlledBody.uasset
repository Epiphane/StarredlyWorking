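; Base player-controlled body that sits on a circle around its owner, the attached planet, before launch.
; While its mesh is not simulating physics, Tick calls SetAngle to place it at ControllerDist from the owner in the XY plane, yawed to the current Angle.
; OnRestore, called on BeginPlay, and OnRemove bind and unbind an event on the orbit player controller's OnLaunch dispatcher.
; Its own OnLaunch function is an empty stub.
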(event EventBeginPlay
  (Class|GravityActor|OnRestore))

(event EventTick
  (params (DeltaSeconds :type Float%20%28single-precision%29))
  ;[1 1 1] Constantly updates position to attached planet pre-launch
  (if (not (Physics|IsSimulatingPhysics (Variables|Default|GetStaticMesh) "None"))
    (CallFunction|SetAngle (Variables|Default|GetAngle))))

(event EventOnRemove
  (bind _asorbit_player_controller_bp (Utilities|Casting|CastToOrbitPlayerControllerBP (Game|GetPlayerController 0)))
  (EventDispatchers|UnbindEventfromOnLaunch _asorbit_player_controller_bp (EventDispatchers|CreateEvent :!event OnLaunch)))

(event EventOnRestore
  (bind _asorbit_player_controller_bp (Utilities|Casting|CastToOrbitPlayerControllerBP (Game|GetPlayerController 0)))
  (EventDispatchers|BindEventtoOnLaunch _asorbit_player_controller_bp (EventDispatchers|CreateEvent :!event OnLaunch)))

(fn ConstructionScript)

(fn SetAngle
  (params (New%20Angle :type Float%20%28double-precision%29))
  (bind _controllerdist (Variables|Default|GetControllerDist))
  (bind _output_get (Variables|Default|SetAngle New%20Angle))
  (Transformation|SetActorLocationAndRotation (+ (Transformation|GetActorLocation (Components|GetOwner)) (Math|Vector|MakeVector (* (Math|Trig|Cos(Degrees) _output_get) _controllerdist) (* _controllerdist (Math|Trig|Sin(Degrees) _output_get)) 0.0)) (Math|Rotator|MakeRotator 0.0 2.7e+02 _output_get)))

(fn OnLaunch)