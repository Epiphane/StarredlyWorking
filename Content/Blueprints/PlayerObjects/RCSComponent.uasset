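; RCSComponent is a fuel-limited reaction control thruster component that rotates its owning player object.
; Rotation input burns fuel over delta time and torques the owner's primitive about its forward axis, scaled by the fuel actually spent.
; It creates a fuel-level widget, manages its HUD slot, and binds to the OrbitPlayerController's launch and reset events.
; Launch refills fuel, while the reset handler's refill and widget removal are disconnected.
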(event Custom|RCS%20Rotation
  (params (Sign :type Float%20%28double-precision%29))
  (if (> (Variables|Default|GetFuel%20Level) 0.0)
    (CallFunction|FireRCS Sign)))

(event EventOnRestore
  (CallFunction|SetHUDSlot "NewEnumerator3" (Variables|Default|GetFuel%20Level%20UI)))

(event EventOnRemove
  (CallFunction|RemovefromHUD "NewEnumerator3" (Variables|Default|GetFuel%20Level%20UI)))

(event EventBeginPlay
  (bind _asorbit_player_controller_bp (Utilities|Casting|CastToOrbitPlayerControllerBP (Game|GetPlayerController 0)))
  (bind _returnvalue (UserInterface|CreateWidget "/Game/Widgets/HUD/WBP_RCSFuelLevel.WBP_RCSFuelLevel_C" _asorbit_player_controller_bp _asorbit_player_controller_bp self))
  (bind _output_get (Variables|Default|SetFuel%20Level%20UI _returnvalue))
  (CallFunction|SetHUDSlot "NewEnumerator3" _output_get)
  (EventDispatchers|BindEventtoOnReset _asorbit_player_controller_bp (EventDispatchers|CreateEvent :!event OnReset))
  (EventDispatchers|BindEventtoOnLaunch _asorbit_player_controller_bp (EventDispatchers|CreateEvent :!event OnLaunch)))

(fn OnReset
  (params (Is%20Full%20Reset :type Boolean)))

(fn OnLaunch
  (Variables|Default|SetFuel%20Level (Variables|Default|GetInitial%20Fuel%20Level)))

(fn FireRCS
  (params (Sign :type Float%20%28double-precision%29))
  (bind _returnvalue (Components|GetOwner))
  ;[1 1 1] Reduce Fuel Level
  (LocalVariables|SetReal%20Amount (- (Variables|Default|GetFuel%20Level) (Math|Float|Max(Float) (- (Variables|Default|GetFuel%20Level) (* (Variables|Default|GetFuel%20Burn%20Rate) (Utilities|Time|GetWorldDeltaSeconds))) 0.0)))
  (Variables|Default|SetFuel%20Level (Math|Float|Max(Float) (- (Variables|Default|GetFuel%20Level) (* (Variables|Default|GetFuel%20Burn%20Rate) (Utilities|Time|GetWorldDeltaSeconds))) 0.0))
  ;[1 1 1] Get vector from actor and apply torque
  (Class|PrimitiveComponent|AddTorqueinDegrees (Actor|GetComponentbyClass _returnvalue "/Script/Engine.PrimitiveComponent") (* (Math|Vector|GetForwardVector (Transformation|GetActorRotation _returnvalue)) (LocalVariables|GetReal%20Amount) (Variables|Default|GetThrust) (* Sign -1.0)) "None" false))