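; Actor component that gives rocket parts fuel-driven thrust and a HUD fuel gauge.
; At BeginPlay it creates the fuel widget and picks a HUD slot by owner class, splitting boosters between two slots by counting existing ones.
; During the simulating stage, Tick burns fuel as up-vector impulses.
; When fuel runs short, non-spaceship owners detach with physics enabled and a velocity kick; reset and launch handlers are empty.
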(event EventOnRestore
  (CallFunction|SetHUDSlot (Variables|Default|GetAssigned%20Slot) (Variables|Default|GetFuel%20Level%20UI)))

(event EventTick
  (params (DeltaSeconds :type Float%20%28single-precision%29))
  (bind _asorbit_player_controller_bp (Utilities|Casting|CastToBP_OrbitPlayerController (Game|GetPlayerController 0)))
  (if (and (Variables|/Game/Blueprints/GameMode/BP_OrbitPlayerController.BP_OrbitPlayerController_C|GetIs%20In%20Simulating%20Stage _asorbit_player_controller_bp) (> (Variables|Default|GetFuel%20Level) 0.0))
    (CallFunction|BurnFuel (* (Variables|Default|GetFuel%20Burn%20Rate) DeltaSeconds))))

(event EventOnRemove
  (CallFunction|RemovefromHUD (Variables|Default|GetAssigned%20Slot) (Variables|Default|GetFuel%20Level%20UI)))

(event EventBeginPlay
  (bind _returnvalue (Components|GetOwner))
  (bind _returnvalue_2 (Utilities|GetClass _returnvalue))
  (bind _asorbit_player_controller_bp (Utilities|Casting|CastToBP_OrbitPlayerController (Game|GetPlayerController 0)))
  (EventDispatchers|BindEventtoOnReset _asorbit_player_controller_bp (EventDispatchers|CreateEvent :!event OnReset))
  (EventDispatchers|BindEventtoOnLaunch _asorbit_player_controller_bp (EventDispatchers|CreateEvent :!event OnLaunch))
  (bind _returnvalue_3 (UserInterface|CreateWidget "/Game/Widgets/HUD/WBP_FuelLevel.WBP_FuelLevel_C" _asorbit_player_controller_bp _asorbit_player_controller_bp self _returnvalue_2))
  (bind _output_get (Variables|Default|SetFuel%20Level%20UI _returnvalue_3))
  (if (== _returnvalue_2 "/Game/Blueprints/PlayerObjects/BP_RocketBooster.BP_RocketBooster_C")
    (bind _outactors (Actor|GetAllActorsOfClass _returnvalue_2))
    (for _array_element _outactors
      (if (!= _array_element (Components|GetOwner))
        (if (Utilities|Enum|Equal(Enum) (Variables|BP_RocketComponent_C|GetAssigned%20Slot (Actor|GetComponentbyClass _array_element "BP_RocketComponent_C")) (Utilities|Enum|LiteralenumE_HUDSlots "NewEnumerator1"))
          (Variables|Default|SetNum%20Originals (+ (Variables|Default|GetNum%20Originals) 1))
          (else
            (Variables|Default|SetNum%20Extras (+ (Variables|Default|GetNum%20Extras) 1))))))
    (if (> (Variables|Default|GetNum%20Originals) (Variables|Default|GetNum%20Extras))
      (bind _output_get_2 (Variables|Default|SetAssigned%20Slot "NewEnumerator5"))
      (CallFunction|SetHUDSlot _output_get_2 _output_get)
      (Development|PrintString "I'm an extra")
      (else
        (bind _output_get_3 (Variables|Default|SetAssigned%20Slot "NewEnumerator1"))
        (CallFunction|SetHUDSlot _output_get_3 _output_get)
        (Development|PrintString "I'm the original")))
    (else
      (bind _output_get_4 (Variables|Default|SetAssigned%20Slot (.Value (Utilities|Map|Find (Variables|Default|GetClass%20To%20HUDSlot%20Map) _returnvalue_2))))
      (CallFunction|SetHUDSlot _output_get_4 _output_get))))

(fn BurnFuel
  (params (Amount :type Float%20%28double-precision%29))
  (bind _returnvalue (Components|GetOwner))
  ;[1 1 1] Reduce Fuel Level
  (if (< (- (Variables|Default|GetFuel%20Level) Amount) 0.0)
    (CallFunction|Detach)
    (else
      (LocalVariables|SetReal%20Amount (- (Variables|Default|GetFuel%20Level) (Math|Float|Max(Float) (- (Variables|Default|GetFuel%20Level) Amount) 0.0)))
      (Variables|Default|SetFuel%20Level (Math|Float|Max(Float) (- (Variables|Default|GetFuel%20Level) Amount) 0.0))
      ;[1 1 1] Get Z vector from actor and apply thrust
      (Physics|AddImpulse (Actor|GetComponentbyClass _returnvalue "/Script/Engine.PrimitiveComponent") (* (Math|Vector|GetUpVector (Transformation|GetActorRotation _returnvalue)) (LocalVariables|GetReal%20Amount) (Variables|Default|GetThrust)) "None" false))))

(fn OnReset
  (params (Is%20Full%20Reset :type Boolean)))

(fn OnLaunch)

(fn Detach
  (bind _returnvalue (Components|GetOwner))
  (bind _returnvalue_2 (Transformation|GetActorRotation _returnvalue))
  (if (!= (Utilities|GetClass _returnvalue) "/Game/Blueprints/PlayerObjects/BP_Spaceship.BP_Spaceship_C")
    (if (not (Variables|Default|GetIs%20Detached))
      (bind _ascontrolled_body (Utilities|Casting|CastToBP_ControlledBody _returnvalue))
      (bind _returnvalue_3 (Physics|GetPhysicsLinearVelocity (Variables|/Game/Blueprints/PlayerObjects/BP_ControlledBody.BP_ControlledBody_C|GetStaticMesh _ascontrolled_body) "None"))
      (Physics|SetSimulatePhysics (Variables|/Game/Blueprints/PlayerObjects/BP_ControlledBody.BP_ControlledBody_C|GetStaticMesh _ascontrolled_body) true)
      (Class|PrimitiveComponent|SetAllPhysicsLinearVelocity (Variables|/Game/Blueprints/PlayerObjects/BP_ControlledBody.BP_ControlledBody_C|GetStaticMesh _ascontrolled_body) (+ _returnvalue_3 (* (Math|Vector|GetUpVector _returnvalue_2) -5e+01) (* (Math|Vector|GetRightVector _returnvalue_2) 1.5e+02)) false)
      (Class|PrimitiveComponent|SetAllPhysicsAngularVelocityinDegrees (Variables|/Game/Blueprints/PlayerObjects/BP_ControlledBody.BP_ControlledBody_C|GetStaticMesh _ascontrolled_body) (Physics|GetPhysicsAngularVelocityinDegrees (Variables|/Game/Blueprints/PlayerObjects/BP_ControlledBody.BP_ControlledBody_C|GetStaticMesh _ascontrolled_body) "None") false)
      (Variables|Default|SetIs%20Detached true))))