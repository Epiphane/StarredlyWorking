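; Actor component that gives a player object a limited fuel supply, burned as thrust during the simulation stage.
; Each Tick while simulating, it drains fuel by burn rate and applies a proportional impulse along the owner's up vector to its primitive component.
; BeginPlay puts a fuel-level widget in a HUD slot and binds to controller reset and launch events.
; The refill and HUD removal logic is disconnected.
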(event EventOnRestore
  (CallFunction|SetHUDSlot "NewEnumerator1" (Variables|Default|GetFuel%20Level%20UI)))

(event EventTick
  (params (DeltaSeconds :type Float%20%28single-precision%29))
  (bind _asorbit_player_controller_bp (Utilities|Casting|CastToOrbitPlayerControllerBP (Game|GetPlayerController 0)))
  (if (and (Variables|/Game/Blueprints/GameMode/OrbitPlayerControllerBP.OrbitPlayerControllerBP_C|GetIs%20In%20Simulating%20Stage _asorbit_player_controller_bp) (> (Variables|Default|GetFuel%20Level) 0.0))
    (CallFunction|BurnFuel (* (Variables|Default|GetFuel%20Burn%20Rate) DeltaSeconds))))

(event EventOnRemove)

(event EventBeginPlay
  (bind _asorbit_player_controller_bp (Utilities|Casting|CastToOrbitPlayerControllerBP (Game|GetPlayerController 0)))
  (bind _returnvalue (UserInterface|CreateWidget "/Game/Widgets/HUD/WBP_FuelLevel.WBP_FuelLevel_C" _asorbit_player_controller_bp _asorbit_player_controller_bp self))
  (bind _output_get (Variables|Default|SetFuel%20Level%20UI _returnvalue))
  (CallFunction|SetHUDSlot "NewEnumerator1" _output_get)
  (EventDispatchers|BindEventtoOnReset _asorbit_player_controller_bp (EventDispatchers|CreateEvent :!event OnReset))
  (EventDispatchers|BindEventtoOnLaunch _asorbit_player_controller_bp (EventDispatchers|CreateEvent :!event OnLaunch)))

(fn BurnFuel
  (params (Amount :type Float%20%28double-precision%29))
  (bind _returnvalue (Components|GetOwner))
  ;[1 1 1] Reduce Fuel Level
  (LocalVariables|SetReal%20Amount (- (Variables|Default|GetFuel%20Level) (Math|Float|Max(Float) (- (Variables|Default|GetFuel%20Level) Amount) 0.0)))
  (Variables|Default|SetFuel%20Level (Math|Float|Max(Float) (- (Variables|Default|GetFuel%20Level) Amount) 0.0))
  ;[1 1 1] Get Z vector from actor and apply thrust
  (Physics|AddImpulse (Actor|GetComponentbyClass _returnvalue "/Script/Engine.PrimitiveComponent") (* (Math|Vector|GetUpVector (Transformation|GetActorRotation _returnvalue)) (LocalVariables|GetReal%20Amount) (Variables|Default|GetThrust)) "None" false))

(fn OnReset
  (params (Is%20Full%20Reset :type Boolean)))

(fn OnLaunch)