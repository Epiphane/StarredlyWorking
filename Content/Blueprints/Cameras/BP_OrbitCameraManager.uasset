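; Player camera manager for an orbit game, supplying a fixed-rotation view that frames a locked object and nearby points of interest.
; Locked and Auto modes merge bounding spheres from two priority sets while within a size threshold, then derive and smoothly interpolate camera position.
; Manual mode follows the pawn directly.
; Controller launch events save the view and switch to Auto; reset events restore it.
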(event Custom|On%20Reset
  (params (Is%20Full%20Reset :type Boolean))
  (Variables|Default|SetCurrent%20Camera%20Location (Variables|Default|GetPrev%20Camera%20Location))
  (Variables|Default|SetCamera%20Mode (Variables|Default|GetPrev%20Camera%20Mode)))

(event Custom|On%20Launch
  (Variables|Default|SetPrev%20Camera%20Location (Variables|Default|GetCurrent%20Camera%20Location))
  (Variables|Default|SetPrev%20Camera%20Mode (Variables|Default|GetCamera%20Mode))
  (bind _position (CallFunction|GetCameraLocation))
  (Variables|Default|SetCurrent%20Camera%20Location _position)
  (Variables|Default|SetCamera%20Mode "NewEnumerator1"))

(event EventTick
  (params (DeltaSeconds :type Float%20%28single-precision%29))
  (CallFunction|PantoCamera DeltaSeconds))

(event EventBeginPlay
  (bind _position (CallFunction|GetCameraLocation))
  (Variables|Default|SetCurrent%20Camera%20Location _position)
  (bind _asbp_orbit_player_controller (Utilities|Casting|CastToBP_OrbitPlayerController (Game|GetPlayerController 0)))
  (EventDispatchers|BindEventtoOnReset _asbp_orbit_player_controller (EventDispatchers|CreateEvent :!event Custom|On%20Reset))
  (EventDispatchers|BindEventtoOnLaunch _asbp_orbit_player_controller (EventDispatchers|CreateEvent :!event Custom|On%20Launch)))

(fn ConstructionScript)

(fn BlueprintUpdateCamera
  (params (CameraTarget :type Actor%20Object%20Reference))
  (return (Variables|Default|GetCurrent%20Camera%20Location) "-90.000000,-90.000000,0.000000" 9e+01 true))

(fn GetActorBoundingSphere
  (params (Actor :type Actor%20Object%20Reference))
  (LocalVariables|SetResult (Utilities|Struct|MakeBoxSphereBounds (Transformation|GetActorLocation Actor) "0, 0, 0" 0.0))
  (for _array_element (Actor|GetComponentsByClass Actor "/Script/Engine.PrimitiveComponent")
    ;[1 1 1] No Splines
    (Utilities|Casting|CastToSplineComponent _array_element
      (:CastFailed
        (if (not (Variables|/Script/Engine.SceneComponent|GetbHiddenInGame _array_element))
          (LocalVariables|SetResult (Class|BoundsHelperFunctions|Combine (LocalVariables|GetResult) (Utilities|Struct|MakeBoxSphereBounds (.Origin (Collision|GetComponentBounds _array_element)) (.BoxExtent (Collision|GetComponentBounds _array_element)) (.SphereRadius (Collision|GetComponentBounds _array_element)))))))))
  (return (LocalVariables|GetResult)))

(fn GetCameraLocation
  (switch Utilities|FlowControl|Switch|SwitchonE_CameraMode (Variables|Default|GetCamera%20Mode)
    (:NewEnumerator0
      _)
    (:NewEnumerator1
      _)
    (:NewEnumerator2
      (return (Transformation|GetActorLocation (Game|Player|GetPlayerPawn 0)) true 0)))
  (bind _locked_object (Variables|Default|GetLocked%20Object)
    (:then
      (LocalVariables|SetViewport%20Bounds (CallFunction|GetActorBoundingSphere _locked_object))
      (LocalVariables|SetBounds%20are%20Valid true))
    (:else
      _))
  (CallFunction|AddPOIstoBounds (Variables|Default|GetPoints%20of%20Interest%20P1) (LocalVariables|GetViewport%20Bounds) (LocalVariables|GetBounds%20are%20Valid) (LocalVariables|GetOutTargets))
  (CallFunction|AddPOIstoBounds (Variables|Default|GetPoints%20of%20Interest%20P2) (LocalVariables|GetViewport%20Bounds) (LocalVariables|GetBounds%20are%20Valid) (LocalVariables|GetOutTargets))
  (return (CallFunction|ViewBoundstoCameraPosition "-90.000000,-90.000000,0.000000" (.origin (LocalVariables|GetViewport%20Bounds)) (Math|Float|Min(Float) (+ (.sphereradius (LocalVariables|GetViewport%20Bounds)) 3e+03 0.0) (Variables|Default|GetPoint%20of%20Interest%20Threshold)) 9e+01) true (LocalVariables|GetOutTargets)))

(fn AddPointOfInterest
  (params (Actor :type Actor%20Object%20Reference) (Priority :type Integer))
  (switch int Priority
    (:Default
      (Utilities|Set|Add (Variables|Default|GetPoints%20of%20Interest%20P1) Actor))
    (:0
      (Utilities|Set|Add (Variables|Default|GetPoints%20of%20Interest%20P2) Actor))))

(fn RemovePointOfInterest
  (params (Actor :type Actor%20Object%20Reference))
  (Utilities|Set|Remove (Variables|Default|GetPoints%20of%20Interest%20P1) Actor)
  (Utilities|Set|Remove (Variables|Default|GetPoints%20of%20Interest%20P2) Actor))

(fn AddPOIstoBounds
  (params (Points%20of%20Interest :type Set%20of%20Actor%20Object%20References) (Bounds :type Box%20Sphere%20Bounds%20Structure%20%28by%20ref%29) (Already%20Valid :type Boolean%20%28by%20ref%29) (Out%20Targets :type Array%20of%20Actor%20Object%20References))
  (bind _result (Utilities|Set|ToArray Points%20of%20Interest))
  (for _array_element _result
    (if Already%20Valid
      (if (<= (.SphereRadius (Math|BoxSphereBounds|BreakBoxSphereBounds (Class|BoundsHelperFunctions|Combine Bounds (CallFunction|GetActorBoundingSphere _array_element)))) (Variables|Default|GetPoint%20of%20Interest%20Threshold))
        (|SetBy-RefVar Bounds (Class|BoundsHelperFunctions|Combine Bounds (CallFunction|GetActorBoundingSphere _array_element)))
        (Utilities|Array|Add Out%20Targets _array_element))
      (else
        (|SetBy-RefVar Bounds (CallFunction|GetActorBoundingSphere _array_element))
        (|SetBy-RefVar Already%20Valid true)
        (Utilities|Array|Add Out%20Targets _array_element)))))

(fn PantoCamera
  (params (Delta%20Time :type Float%20%28single-precision%29))
  (Utilities|FlowControl|Sequence
    (:then_0
      (bind _locked_object (Variables|Default|GetLocked%20Object)
        (:then
          (LocalVariables|SetIs%20Player%20in%20Viewport (CallFunction|IsPointinViewport (Transformation|GetActorLocation _locked_object) 1e+03)))
        (:else
          (LocalVariables|SetIs%20Player%20in%20Viewport true))))
    (:then_1
      (bind (_position _use_position _targets) (CallFunction|GetCameraLocation))
      (if _use_position
        (switch Utilities|FlowControl|Switch|SwitchonE_CameraMode (Variables|Default|GetCamera%20Mode)
          (:NewEnumerator0
            (Variables|Default|SetCurrent%20Camera%20Location (Math|Interpolation|VInterpTo (Variables|Default|GetCurrent%20Camera%20Location) _position Delta%20Time (Math|Float|SelectFloat 7.0 7.0 (Math|Boolean|ANDBoolean (> (Math|Vector|Distance(Vector) (Variables|Default|GetCurrent%20Camera%20Location) _position) 1e+04) (LocalVariables|GetIs%20Player%20in%20Viewport) (> (Utilities|Array|Length _targets) 1)))) :!label _label))
          (:NewEnumerator1
            (goto _label))
          (:NewEnumerator2
            (Variables|Default|SetCurrent%20Camera%20Location _position)))))))