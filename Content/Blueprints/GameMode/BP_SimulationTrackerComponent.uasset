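; Actor component that records its owner's simulation history so BP_OrbitPlayerController can scrub through time and resume from any recorded frame.
; While simulating, each tick stores transform, velocities, rocket and RCS fuel, and attachment state in an array indexed by SimTime.
; Time updates move the owner along that history, hiding it before its first frame.
; Resuming restores saved state and overwrites later frames, or destroys still-hidden owners.
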(event EventBeginPlay
  (bind _returnvalue (Components|GetOwner))
  (Variables|Default|SetParent%20Reference _returnvalue)
  (Variables|Default|SetParent%20Static%20Mesh (Actor|GetComponentbyClass _returnvalue "/Script/Engine.StaticMeshComponent"))
  (bind _asbp_orbit_player_controller (Utilities|Casting|CastToBP_OrbitPlayerController (Game|GetPlayerController 0)))
  (EventDispatchers|BindEventtoOnReset _asbp_orbit_player_controller (EventDispatchers|CreateEvent :!event OnReset))
  (EventDispatchers|BindEventtoOnTimeUpdate _asbp_orbit_player_controller (EventDispatchers|CreateEvent :!event OnTimeUpdate)))

(event EventTick
  (params (DeltaSeconds :type Float%20%28single-precision%29))
  (bind _parent_reference (Variables|Default|GetParent%20Reference))
  (bind _sim_time_param_array (Variables|Default|GetSim%20Time%20Param%20Array))
  (bind _asbp_orbit_player_controller (Utilities|Casting|CastToBP_OrbitPlayerController (Game|GetPlayerController 0)))
  (if (Variables|/Game/Blueprints/GameMode/BP_OrbitPlayerController.BP_OrbitPlayerController_C|GetIs%20In%20Simulating%20Stage _asbp_orbit_player_controller)
    (if (Variables|Default|GetIs%20Tracking)
      (Variables|Default|SetSim%20Time (+ (Variables|Default|GetSim%20Time) 1))
      (CallFunction|GetAllParams :!label _label)
      (Variables|Default|SetIs%20Tracking true)
      (elif (Utilities|Array|IsValidIndex _sim_time_param_array (Variables|Default|GetSim%20Time))
        (CallFunction|SetRocketParams (Utilities|Array|Get(acopy) _sim_time_param_array (Variables|Default|GetSim%20Time)))
        (CallFunction|SetRCSParams (Utilities|Array|Get(acopy) _sim_time_param_array (Variables|Default|GetSim%20Time)))
        (CallFunction|SetActorVelocity (Utilities|Array|Get(acopy) _sim_time_param_array (Variables|Default|GetSim%20Time)))
        (goto _label)
        (elif (Variables|/Script/Engine.Actor|GetbHidden _parent_reference)
          (Actor|DestroyActor _parent_reference)
          (else
            (goto _label)))))
    (else
      (Variables|Default|SetIs%20Tracking false))))

(fn OnReset
  (params (Is%20Full%20Reset :type Boolean))
  (Variables|Default|SetSim%20Time 0)
  (Utilities|Array|Clear (Variables|Default|GetSim%20Time%20Param%20Array)))

(fn OnTimeUpdate
  (params (Time%20Sign :type Float%20%28double-precision%29))
  (bind _sim_time_param_array (Variables|Default|GetSim%20Time%20Param%20Array))
  (bind _parent_reference (Variables|Default|GetParent%20Reference))
  (if (>= (+ (Math|Float|Truncate Time%20Sign) (Variables|Default|GetSim%20Time)) 0)
    (if (< (+ (Math|Float|Truncate Time%20Sign) (Variables|Default|GetSim%20Time)) (Variables|Default|GetSim%20Time%20Limit))
      (if (Utilities|Array|IsValidIndex _sim_time_param_array (+ (Math|Float|Truncate Time%20Sign) (Variables|Default|GetSim%20Time)))
        (Transformation|SetActorLocationAndRotation (Variables|Default|GetParent%20Reference) (.Position (Utilities|Struct|BreakF_SimTimeStruct (Utilities|Array|Get(acopy) _sim_time_param_array (+ (Math|Float|Truncate Time%20Sign) (Variables|Default|GetSim%20Time))))) (.Rotation (Utilities|Struct|BreakF_SimTimeStruct (Utilities|Array|Get(acopy) _sim_time_param_array (+ (Math|Float|Truncate Time%20Sign) (Variables|Default|GetSim%20Time))))))
        (Rendering|SetActorHiddenInGame _parent_reference false)
        (Variables|Default|SetSim%20Time (+ (Math|Float|Truncate Time%20Sign) (Variables|Default|GetSim%20Time)) :!label _label)))
    (else
      (Rendering|SetActorHiddenInGame _parent_reference true)
      (goto _label))))

(fn SetRocketParams
  (params (Inputs :type F%20Sim%20Time%20Struct%20Structure))
  (bind (_position _rotation _linearvelocity _angularvelocity _rocketfuellevel _rcsfuellevel _isdetatched _rocketsocketname) (Utilities|Struct|BreakF_SimTimeStruct Inputs))
  (bind _parent_reference (Variables|Default|GetParent%20Reference))
  (bind _parent_reference_2 (Variables|Default|GetParent%20Reference))
  (bind _returnvalue (Actor|GetComponentbyClass _parent_reference "/Game/Blueprints/PlayerObjects/BP_RocketComponent.BP_RocketComponent_C"))
  (bind _returnvalue_2 (Components|GetOwner _parent_reference_2))
  (Utilities|IsValid _returnvalue
    (:Is%20Valid
      (Variables|/Game/Blueprints/PlayerObjects/BP_RocketComponent.BP_RocketComponent_C|SetFuel%20Level _returnvalue _rocketfuellevel)
      (bind _output_get (Variables|/Game/Blueprints/PlayerObjects/BP_RocketComponent.BP_RocketComponent_C|SetIs%20Detached _returnvalue _isdetatched))
      (if _output_get
        (Development|PrintString "Detached")
        (elif (!= _rocketsocketname "")
          (Development|PrintString (Utilities|String|Append "Rocket " (Utilities|GetDisplayName _parent_reference_2) "should attach to " (Utilities|GetDisplayName _returnvalue_2) "at socket " (Utilities|String|ToString(Name) _rocketsocketname)))
          (Transformation|AttachActorToActor _parent_reference_2 _returnvalue_2 _rocketsocketname "SnapToTarget" "SnapToTarget" "KeepWorld" true))))))

(fn SetRCSParams
  (params (Inputs :type F%20Sim%20Time%20Struct%20Structure))
  (bind _parent_reference (Variables|Default|GetParent%20Reference))
  (bind _returnvalue (Actor|GetComponentbyClass _parent_reference "/Game/Blueprints/PlayerObjects/BP_RCSComponent.BP_RCSComponent_C"))
  (Utilities|IsValid _returnvalue
    (:Is%20Valid
      (Variables|/Game/Blueprints/PlayerObjects/BP_RCSComponent.BP_RCSComponent_C|SetFuel%20Level _returnvalue (.RCSFuelLevel (Utilities|Struct|BreakF_SimTimeStruct Inputs))))))

(fn SetActorVelocity
  (params (Inputs :type F%20Sim%20Time%20Struct%20Structure))
  (bind (_position _rotation _linearvelocity _angularvelocity) (Utilities|Struct|BreakF_SimTimeStruct Inputs))
  (Utilities|IsValid (Actor|GetAttachParentActor (Variables|Default|GetParent%20Reference))
    (:Is%20Not%20Valid
      (Physics|AddImpulse (Variables|Default|GetParent%20Static%20Mesh) _linearvelocity "None" true)
      (Class|PrimitiveComponent|SetPhysicsAngularVelocityinDegrees (Variables|Default|GetParent%20Static%20Mesh) _angularvelocity false "None"))))

(fn GetAllParams
  (bind _parent_reference (Variables|Default|GetParent%20Reference))
  (bind _sim_time_param_array (Variables|Default|GetSim%20Time%20Param%20Array))
  (bind _parent_reference_2 (Variables|Default|GetParent%20Reference))
  (bind _returnvalue (Actor|GetComponentbyClass _parent_reference "/Game/Blueprints/PlayerObjects/BP_RocketComponent.BP_RocketComponent_C"))
  (bind _returnvalue_2 (Actor|GetComponentbyClass _parent_reference "/Game/Blueprints/PlayerObjects/BP_RCSComponent.BP_RCSComponent_C"))
  (Utilities|IsValid _returnvalue
    (:Is%20Valid
      ;[1 0 0] Better way to do this?
      (bind _output_get (LocalVariables|SetValid%20Rocket%20Fuel (Variables|/Game/Blueprints/PlayerObjects/BP_RocketComponent.BP_RocketComponent_C|GetFuel%20Level _returnvalue)))
      (bind _output_get_2 (LocalVariables|SetValid%20Is%20Detached (Variables|/Game/Blueprints/PlayerObjects/BP_RocketComponent.BP_RocketComponent_C|GetIs%20Detached _returnvalue)))
      (bind _output_get_3 (LocalVariables|SetValid%20Socket%20Name (Variables|/Game/Blueprints/PlayerObjects/BP_RocketComponent.BP_RocketComponent_C|GetAttachment%20Socket _returnvalue))))
    (:Is%20Not%20Valid
      _))
  (Utilities|IsValid _returnvalue_2
    (:Is%20Valid
      (bind _output_get_4 (LocalVariables|SetValid%20RCS%20Fuel (Variables|/Game/Blueprints/PlayerObjects/BP_RCSComponent.BP_RCSComponent_C|GetFuel%20Level _returnvalue_2))))
    (:Is%20Not%20Valid
      _))
  (bind _returnvalue_3 (Physics|GetPhysicsLinearVelocity (Variables|Default|GetParent%20Static%20Mesh) "None"))
  (if (Utilities|Array|IsValidIndex _sim_time_param_array (Variables|Default|GetSim%20Time))
    (Utilities|Array|SetArrayElem _sim_time_param_array (Variables|Default|GetSim%20Time) (Utilities|Struct|MakeF_SimTimeStruct (Transformation|GetActorLocation _parent_reference_2) (Transformation|GetActorRotation _parent_reference_2) _returnvalue_3 (Physics|GetPhysicsAngularVelocityinDegrees (Variables|Default|GetParent%20Static%20Mesh) "None") _output_get _output_get_4 _output_get_2 _output_get_3))
    (else
      (bind _returnvalue_4 (Utilities|Array|Add _sim_time_param_array (Utilities|Struct|MakeF_SimTimeStruct (Transformation|GetActorLocation _parent_reference_2) (Transformation|GetActorRotation _parent_reference_2) _returnvalue_3 (Physics|GetPhysicsAngularVelocityinDegrees (Variables|Default|GetParent%20Static%20Mesh) "None") _output_get _output_get_4 _output_get_2 _output_get_3)))
      (Variables|Default|SetSim%20Time _returnvalue_4)))
  (Variables|Default|SetSim%20Time%20Limit (Variables|Default|GetSim%20Time)))