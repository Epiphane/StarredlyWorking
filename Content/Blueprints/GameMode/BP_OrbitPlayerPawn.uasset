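; Orbit-camera player pawn that plays a one-time cinematic intro per level, tracked in a save game.
; On first visit, a timeline lerps it from above the spaceship to the BP_InitialCamera transform, then marks the level done and starts the controller's preview.
; On later visits it snaps straight to that transform.
; A controller reset skips a running intro to its end; zoom input adjusts spring arm length.
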(event Custom|On%20Reset
  (params (Is%20Full%20Reset :type Boolean))
  (CallFunction|CancelIntro))

(event Custom|Cancel%20Intro
  (Utilities|FlowControl|Sequence
    (:then_0
      (if (Audio|Components|Audio|IsPlaying (Variables|Default|GetPan%20Camera%20Out))
        (Transformation|SetActorTransform (Variables|Default|GetEnd%20Cinematic%20Transform))
        (CallFunction|SetCurrentLevelIntroComplete true :!label _label)
        (Default|BeginPreview (stale EventBeginPlay _asbp_orbit_player_controller))))
    (:then_1
      (bind _progress (Timeline|Pan%20Camera%20Out Stop)
        (:Update
          (Transformation|SetActorTransform (Math|Transform|Lerp(Transform) (Variables|Default|GetStart%20Cinematic%20Transform) (Variables|Default|GetEnd%20Cinematic%20Transform) _progress)))
        (:Finished
          (goto _label))))))

(event Custom|Perform%20Cinematic%20Intro
  (bind _returnvalue (CallFunction|GetStartCameraPosition))
  (Variables|Default|SetEnd%20Cinematic%20Transform _returnvalue)
  (bind _returnvalue_2 (Actor|GetActorOfClass "/Game/Blueprints/PlayerObjects/BP_Spaceship.BP_Spaceship_C"))
  (Utilities|IsValid _returnvalue_2
    (:Is%20Valid
      (Variables|Default|SetStart%20Cinematic%20Transform (Math|Transform|MakeTransform (+ (.location (Transformation|GetActorTransform _returnvalue_2)) (Math|Vector|MakeVector 0.0 0.0 1e+03)) (Math|Rotator|FindLookatRotation (+ (.location (Transformation|GetActorTransform _returnvalue_2)) (Math|Vector|MakeVector 0.0 0.0 1e+03)) (.location (Transformation|GetActorTransform _returnvalue_2))) "1.000000,1.000000,1.000000"))
      (bind _progress (Timeline|Pan%20Camera%20Out Play)
        (:Update
          (Transformation|SetActorTransform (Math|Transform|Lerp(Transform) (Variables|Default|GetStart%20Cinematic%20Transform) (Variables|Default|GetEnd%20Cinematic%20Transform) _progress)))
        (:Finished
          (CallFunction|SetCurrentLevelIntroComplete true)
          (Default|BeginPreview (stale EventBeginPlay _asbp_orbit_player_controller)))))))

(event Input|EnhancedActionEvents|EnhancedInputActionIA_Zoom
  (params (ActionValue :type Float%20%28double-precision%29) (ElapsedSeconds :type Float%20%28double-precision%29) (TriggeredSeconds :type Float%20%28double-precision%29) (InputAction :type Input%20Action%20Object%20Reference :default "/Game/Input/IA_Zoom.IA_Zoom"))
  (bind _springarm (Variables|Default|GetSpringArm))
  (Variables|/Script/Engine.SpringArmComponent|SetTargetArmLength _springarm (+ (Variables|/Script/Engine.SpringArmComponent|GetTargetArmLength _springarm) (* ActionValue -5e+02))))

(event EventBeginPlay
  (Utilities|FlowControl|Sequence
    (:then_0
      (bind _asbp_orbit_player_controller (Utilities|Casting|CastToBP_OrbitPlayerController (Pawn|GetController)))
      (EventDispatchers|AssignOnReset _asbp_orbit_player_controller (delegate Custom|On%20Reset)))
    (:then_1
      (CallFunction|LoadSaveState)
      (bind _returnvalue (Game|GetCurrentLevelName true))
      (if (.Value (Utilities|Map|Find (Variables|/Game/Blueprints/GameMode/BP_CinematicIntroSaveGame.BP_CinematicIntroSaveGame_C|GetDid%20Intro%20Cinematic%20Run (Variables|Default|GetIntro%20Save%20Settings)) _returnvalue))
        (bind _returnvalue_2 (CallFunction|GetStartCameraPosition))
        (bind _output_get (Variables|Default|SetEnd%20Cinematic%20Transform _returnvalue_2))
        (Transformation|SetActorTransform _output_get)
        (else
          (CallFunction|PerformCinematicIntro))))))

(fn ConstructionScript)

(fn LoadSaveState
  (bind _save_slot (Variables|Default|GetSave%20Slot))
  (bind _returnvalue (SaveGame|LoadGamefromSlot _save_slot))
  (bind _asbp_cinematic_intro_save_game (Utilities|Casting|CastToBP_CinematicIntroSaveGame _returnvalue)
    (:then
      (Variables|Default|SetIntro%20Save%20Settings _asbp_cinematic_intro_save_game))
    (:CastFailed
      (bind _returnvalue_2 (SaveGame|CreateSaveGameObject "/Game/Blueprints/GameMode/BP_CinematicIntroSaveGame.BP_CinematicIntroSaveGame_C"))
      (SaveGame|SaveGametoSlot _returnvalue_2 _save_slot))))

(fn SaveState
  (SaveGame|SaveGametoSlot (Variables|Default|GetIntro%20Save%20Settings) (Variables|Default|GetSave%20Slot)))

(fn SetCurrentLevelIntroComplete
  (params (Value :type Boolean))
  (bind _returnvalue (Game|GetCurrentLevelName true))
  (Utilities|Map|Add (Variables|/Game/Blueprints/GameMode/BP_CinematicIntroSaveGame.BP_CinematicIntroSaveGame_C|GetDid%20Intro%20Cinematic%20Run (Variables|Default|GetIntro%20Save%20Settings)) _returnvalue Value)
  (CallFunction|SaveState))

(fn GetStartCameraPosition
  (bind _returnvalue (Actor|GetActorOfClass "/Game/Blueprints/Cameras/BP_InitialCamera.BP_InitialCamera_C"))
  (return (Transformation|GetActorTransform (select (Utilities|IsValid _returnvalue) _returnvalue self))))