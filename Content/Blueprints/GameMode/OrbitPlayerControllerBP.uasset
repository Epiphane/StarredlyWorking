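; Player controller for an orbital launch game that switches the level between a planning stage and a physics simulation stage.
; BeginPlay creates the time UI, pauses physics and plays a preview timeline that broadcasts simulation time to TimeBasedObject actors; SetTime stops it to scrub manually.
; Launch enables the gravity subsystem and body physics, while reset functions return to planning.
; It also adjusts spaceship launch angle from input and sets initial fuel.
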(event Input|EnhancedActionEvents|EnhancedInputActionIA_Movement
  (params (ActionValue :type Vector%202D%20Structure) (ElapsedSeconds :type Float%20%28double-precision%29) (TriggeredSeconds :type Float%20%28double-precision%29) (InputAction :type Input%20Action%20Object%20Reference :default "/Game/Input/IA_Movement.IA_Movement"))
  (bind _outactors (Actor|GetAllActorsOfClass "/Game/Blueprints/Spaceship.Spaceship_C"))
  (for _array_element _outactors
    (Default|ModifyLaunchAngle _array_element (* (.x ActionValue) TriggeredSeconds))))

(event EventBeginPlay
  (bind _self self)
  (Utilities|FlowControl|Sequence
    (:then_0
      (bind _returnvalue (UserInterface|CreateWidget "/Game/Widgets/Widget_TimeUI.Widget_TimeUI_C" _self _self))
      (UserInterface|Viewport|AddtoViewport _returnvalue 0)
      (Variables|Default|SetPlayer%20UI _returnvalue))
    (:then_1
      (CallFunction|PausePhysics))
    (:then_2
      (Input|AddMappingContext (PlayerController|LocalPlayerSubsystems|GetEnhancedInputLocalPlayerSubsystem) "/Game/Input/IM_GameControls.IM_GameControls" 0 "(bIgnoreAllPressedKeysUntilRelease=True,bForceImmediately=False,bNotifyUserSettings=False)"))
    (:then_3
      (bind _time (Timeline|Level%20Preview Play)
        (:Update
          (Variables|Default|SetSimulationTime _time)
          (bind _outactors (Actor|GetAllActorswithInterface "/Script/StarredlyWorking.TimeBasedObject"))
          (for _array_element _outactors
            (if (!= _array_element self)
              (Class|TimeBasedObject|SetTime(Message) _array_element (stale EventSetTime _output_get)))))
        (:Finished
          (Class|TimeBasedObject|SetTime 0.0))))))

(event EventSetTime
  (params (CurrentTime :type Float%20%28single-precision%29))
  (bind _output_get (Variables|Default|SetSimulationTime CurrentTime))
  (Audio|Components|Audio|Stop (Variables|Default|GetLevel%20Preview))
  (bind _asorbit_player_pawn_bp (Utilities|Casting|CastToOrbitPlayerPawnBP (Game|Player|GetPlayerPawn 0))
    (:then
      (Default|CancelIntro _asorbit_player_pawn_bp))
    (:CastFailed
      _))
  (bind _outactors (Actor|GetAllActorswithInterface "/Script/StarredlyWorking.TimeBasedObject"))
  (for _array_element _outactors
    (if (!= _array_element self)
      (Class|TimeBasedObject|SetTime(Message) _array_element _output_get))))

(fn ConstructionScript)

(fn PartialReset
  ;[1 1 1] Reset Positions
  (bind _outactors (Actor|GetAllActorsOfClass "/Game/Blueprints/ControlledBody.ControlledBody_C"))
  (for _array_element _outactors
    (Default|SetAngle _array_element (Variables|/Game/Blueprints/ControlledBody.ControlledBody_C|GetAngle _array_element)))
  (CallFunction|PausePhysics)
  ;[1 1 1] Resume Physics
  (bind _outactors_2 (Actor|GetAllActorsOfClass "/Game/Blueprints/SimulatedBody.SimulatedBody_C"))
  (for _array_element_2 _outactors_2
    (Class|TimeBasedObject|SetTime _array_element_2 (Variables|Default|GetSimulationTime)))
  (Default|CallOnReset false))

(fn Reset
  (params (Full%20Reset :type Boolean))
  ;[1 1 1] Destroy each ControlledBody
  (bind _outactors (Actor|GetAllActorsOfClass "/Game/Blueprints/ControlledBody.ControlledBody_C"))
  (for _array_element _outactors
    (Actor|DestroyActor _array_element)
    (CallFunction|PausePhysics)
    (Class|TimeBasedObject|SetTime 0.0)
    (Default|CallOnReset Full%20Reset)))

(fn PausePhysics
  (Variables|Default|SetIs%20In%20Simulating%20Stage false)
  (Variables|Default|SetIs%20In%20Planning%20Stage true)
  (Class|GravitySubsystem|SetEnabled (Subsystems|GetGravitySubsystem) false)
  ;[1 1 1] Pause each SimulatedBody
  (bind _outactors (Actor|GetAllActorsOfClass "/Game/Blueprints/SimulatedBody.SimulatedBody_C"))
  (for _array_element _outactors
    (Physics|SetSimulatePhysics (Variables|/Game/Blueprints/SimulatedBody.SimulatedBody_C|GetStaticMesh _array_element) false))
  ;[1 1 1] Pause each ControlledBody
  (bind _outactors_2 (Actor|GetAllActorsOfClass "/Game/Blueprints/ControlledBody.ControlledBody_C"))
  (for _array_element_2 _outactors_2
    (Physics|SetSimulatePhysics (Variables|/Game/Blueprints/ControlledBody.ControlledBody_C|GetStaticMesh _array_element_2) false)))

(fn UnpausePhysics
  (Variables|Default|SetIs%20In%20Simulating%20Stage true)
  (Variables|Default|SetIs%20In%20Planning%20Stage false)
  (Class|GravitySubsystem|SetEnabled (Subsystems|GetGravitySubsystem) true)
  (bind _outactors (Actor|GetAllActorsOfClass "/Game/Blueprints/SimulatedBody.SimulatedBody_C"))
  (for _array_element _outactors
    (Physics|SetSimulatePhysics (Variables|/Game/Blueprints/SimulatedBody.SimulatedBody_C|GetStaticMesh _array_element) true)))

(fn Launch
  (CallFunction|UnpausePhysics)
  (bind _outactors (Actor|GetAllActorsOfClass "/Game/Blueprints/SimulatedBody.SimulatedBody_C"))
  (for _array_element _outactors
    (Class|TimeBasedObject|SetTime _array_element (Variables|Default|GetSimulationTime))
    (Audio|Components|Audio|Stop (Variables|Default|GetLevel%20Preview)))
  (Default|CallOnLaunch))

(fn SetFuelLevels
  (params (Fuel%20Levels :type Array%20of%20Floats%20%28double-precision%29))
  (bind _outactors (Actor|GetAllActorsOfClass "/Game/Blueprints/Spaceship.Spaceship_C"))
  (for _array_element _outactors
    (Variables|/Game/Blueprints/FuelComponent.FuelComponent_C|SetInitial%20Fuel%20Level (Actor|GetComponentbyClass _array_element "/Game/Blueprints/FuelComponent.FuelComponent_C") (Utilities|Array|Get(acopy) Fuel%20Levels))))