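; Blueprint function library of shortcuts to player 0's orbit controller and camera manager, plus view-bounds math.
; HUD slot and point-of-interest helpers cast and forward calls, doing nothing if the cast fails.
; View bounds project along camera forward, using camera height as distance and FOV and aspect ratio for size, feeding a margin-padded XY point-in-view test.
; A reverse helper derives camera position from bounds using an unexplained 1.8 factor.
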(fn SetHUDSlot
  (params (Slot :type E_HUDSlots%20Enum :default "NewEnumerator0") (Content :type User%20Widget%20Object%20Reference))
  (bind _asbp_orbit_player_controller (Utilities|Casting|CastToBP_OrbitPlayerController (Game|GetPlayerController (LocalVariables|Get__WorldContext))))
  (Default|SetHUDSlot _asbp_orbit_player_controller Slot Content))

(fn RemovefromHUD
  (params (Slot :type E_HUDSlots%20Enum :default "NewEnumerator0") (Content :type User%20Widget%20Object%20Reference))
  (bind _asbp_orbit_player_controller (Utilities|Casting|CastToBP_OrbitPlayerController (Game|GetPlayerController (LocalVariables|Get__WorldContext))))
  (Default|RemoveHUDSlot _asbp_orbit_player_controller Slot Content))

(fn GetPlayerViewBounds
  (bind ___worldcontext (LocalVariables|Get__WorldContext))
  (bind ___worldcontext_2 (LocalVariables|Get__WorldContext))
  (bind _returnvalue (Viewport|GetViewportSize ___worldcontext_2))
  (bind _returnvalue_2 (Game|GetPlayerCameraManager ___worldcontext))
  (bind _returnvalue_3 (Camera|GetFOVAngle _returnvalue_2))
  (bind _returnvalue_4 (Camera|GetCameraLocation _returnvalue_2))
  (bind _returnvalue_5 (Math|Trig|DegreesToRadians _returnvalue_3))
  (bind _z (Math|Vector|BreakVector _returnvalue_4))
  (bind _returnvalue_6 (* _returnvalue_5 0.5))
  (bind _returnvalue_7 (Math|Trig|Tan(Radians) _returnvalue_6))
  (bind _returnvalue_8 (* _z _returnvalue_7))
  ;[1 1 1] https://forums.unrealengine.com/t/how-to-get-a-cameras-frustum-plane-at-a-specific-distance-if-possible-in-bp/556232
  (return (+ (* (Math|Vector|GetForwardVector (Camera|GetCameraRotation _returnvalue_2)) _z) _returnvalue_4) (Math|Vector2D|MakeVector2D (/ (* _returnvalue_8 (/ (.x _returnvalue) (.y _returnvalue))) 1.0) (/ _returnvalue_8 1.0))))

(fn IsPointinViewport
  (params (Point :type Vector) (Margin :type Float%20%28double-precision%29))
  (bind ___worldcontext (LocalVariables|Get__WorldContext))
  (bind (_center _half_size) (CallFunction|GetPlayerViewBounds ___worldcontext))
  (bind _result (Math|Float|NegateFloat Margin)
    (:%20%20
      (return (and (and (>= (+ (.x _center) (.x _half_size) _result) (.x Point)) (>= (.x Point) (Utilities|Operators|Subtract (.x _center) (.x _half_size) _result))) (and (>= (+ (.y _center) (.y _half_size) _result) (.y Point)) (>= (.y Point) (Utilities|Operators|Subtract (.y _center) (.y _half_size) _result))))))))

(fn ViewBoundstoCameraPosition
  (params (Rotation :type Rotator) (Center :type Vector) (Half%20Size%20Y :type Float%20%28double-precision%29) (FOV :type Float%20%28double-precision%29))
  (return (- Center (* (Math|Vector|GetForwardVector Rotation) (/ (* Half%20Size%20Y 1.8) (Math|Trig|Tan(Radians) (* (Math|Trig|DegreesToRadians FOV) 0.5)))))))

(fn AddPointOfInterest
  (params (Actor :type Actor%20Object%20Reference) (Priority :type Integer))
  (bind _asbp_orbit_camera_manager (Utilities|Casting|CastToBP_OrbitCameraManager (Game|GetPlayerCameraManager (LocalVariables|Get__WorldContext))))
  (Default|AddPointOfInterest _asbp_orbit_camera_manager Actor Priority))

(fn RemovePointOfInterest
  (params (Actor :type Actor%20Object%20Reference))
  (bind _asbp_orbit_camera_manager (Utilities|Casting|CastToBP_OrbitCameraManager (Game|GetPlayerCameraManager (LocalVariables|Get__WorldContext))))
  (Default|RemovePointOfInterest _asbp_orbit_camera_manager Actor))